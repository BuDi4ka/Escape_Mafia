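; BP_Intercom_Dick_New is a hint-system intercom that shows a prompt widget and outline on overlap and plays a camera shutter sound on interact.
; Two fast looping timers refresh the prompt and copy availability from the Donny intercoms' cooldown, with the last one checked deciding Interactable.
; Sphere overlaps set the prompt flags.
; IsInteractable always returns false, and Tick debug-prints the Interactable flag.
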(event OnComponentBeginOverlap(Sphere)
  (params (OverlappedComponent :type Primitive%20Component%20Object%20Reference) (OtherActor :type Actor%20Object%20Reference) (OtherComp :type Primitive%20Component%20Object%20Reference) (OtherBodyIndex :type Integer) (bFromSweep :type Boolean) (SweepResult :type Hit%20Result%20Structure%20%28by%20ref%29))
  (Variables|Default|SetShowInteract true)
  (if (Variables|Default|GetInteractable)
    (Variables|Default|SetisPrompt true)
    (Rendering|SetVisibility (Variables|Default|GetWidget) true false)
    (Rendering|Material|SetOverlayMaterial (Variables|Default|GetStaticMesh) "/Game/Assets/Materials/M_Outline.M_Outline" :!class /Script/Engine.MeshComponent)))

(event OnComponentEndOverlap(Sphere)
  (params (OverlappedComponent :type Primitive%20Component%20Object%20Reference) (OtherActor :type Actor%20Object%20Reference) (OtherComp :type Primitive%20Component%20Object%20Reference) (OtherBodyIndex :type Integer))
  (Variables|Default|SetShowInteract false)
  (if (Variables|Default|GetInteractable)
    (Variables|Default|SetisPrompt false)
    (Rendering|SetVisibility (Variables|Default|GetWidget) false false)
    (Rendering|Material|SetOverlayMaterial (Variables|Default|GetStaticMesh) 0 :!class /Script/Engine.MeshComponent)))

(event Custom|CheckDonnyCooldown
  (for _array_element (Variables|Default|GetDonny%20Intercom%20)
    (if (Variables|/Game/Items/Hint_System/BP_Intercom_Donny_New.BP_Intercom_Donny_New_C|GetisCooldown _array_element)
      (Variables|Default|SetInteractable false)
      (else
        (Variables|Default|SetInteractable true)))))

(event Custom|CheckWidget
  (bind _staticmesh (Variables|Default|GetStaticMesh))
  (bind _widget (Variables|Default|GetWidget))
  (if (Math|Boolean|ANDBoolean (Variables|Default|GetInteractable) (Variables|Default|GetisPrompt) (Variables|Default|GetShowInteract))
    (Rendering|SetVisibility _widget true false)
    (Rendering|Material|SetOverlayMaterial _staticmesh "/Game/Assets/Materials/M_Outline.M_Outline" :!class /Script/Engine.MeshComponent)
    (else
      (Rendering|SetVisibility _widget false false)
      (Rendering|Material|SetOverlayMaterial _staticmesh 0 :!class /Script/Engine.MeshComponent))))

(event EventTick
  (params (DeltaSeconds :type Float%20%28single-precision%29))
  (|CallParentFunction DeltaSeconds)
  (Development|PrintString (Utilities|String|ToString(Boolean) (Variables|Default|GetInteractable))))

(event EventBeginPlay
  (bind _outactors (Actor|GetAllActorsOfClass "/Game/Items/Hint_System/BP_Intercom_Donny_New.BP_Intercom_Donny_New_C"))
  (Variables|Default|SetDonny%20Intercom%20 _outactors)
  (Utilities|Time|SetTimerbyEvent (delegate Custom|CheckDonnyCooldown) 0.01 true)
  (Utilities|Time|SetTimerbyEvent (delegate Custom|CheckWidget) 0.01 true))

(event EventOnInteract
  (params (InteractingPlayer :type Character%20Object%20Reference) (Player%20Index :type Integer))
  (bind _returnvalue (Audio|SpawnSound2D "/Engine/VREditor/Sounds/UI/Camera_Shutter.Camera_Shutter" 1.0 1.0 0.0 0))
  (Audio|Components|Audio|StopDelayed _returnvalue 1.0))

(fn ConstructionScript
  (|CallParentFunction))

(fn IsInteractable
  (return false))