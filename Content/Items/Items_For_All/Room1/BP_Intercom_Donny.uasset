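; BP_Intercom_Donny is an interactable intercom in Room1 that acts as one step in a chained intercom sequence.
; On BeginPlay it finds the tagged BP_Intercom_Dick actor and caches it.
; When used while enabled, it spawns BP_Book_ForIntercom at a hardcoded location, enables Dick's intercom and disables itself, so it works only once until re-enabled.
; Both outcomes print debug strings, and IsInteractable reports its Interactable flag.
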(event EventBeginPlay
  (bind _outactors (Actor|GetAllActorsOfClasswithTag "/Game/Items/Items_For_All/Room1/BP_Intercom_Dick.BP_Intercom_Dick_C" "dickintercom"))
  (for _array_element _outactors
    (Variables|Default|SetIntercom%20Dick _array_element)))

(event EventOnIntercom
  (params (IntercomPlayer :type Character%20Object%20Reference))
  (if (Variables|Default|GetcanIntercom)
    (Game|SpawnActorfromClass "/Game/Items/Items_For_Intercom/Room1/BP_Book_ForIntercom.BP_Book_ForIntercom_C" (Math|Transform|MakeTransform "700.000000,-1024.014545,30.000000" "0, 0, 0" "1.000000,1.000000,1.000000") "Undefined" "MultiplyWithRoot" 0 0)
    (Development|PrintString "Intercom Donny Interacted " true true "(R=0.000000,G=0.012252,B=0.244792,A=1.000000)")
    (Variables|/Game/Items/Items_For_All/Room1/BP_Intercom_Dick.BP_Intercom_Dick_C|SetcanIntercom (Variables|Default|GetIntercom%20Dick) true)
    (Variables|Default|SetcanIntercom false)
    (else
      (Development|PrintString "CAN NOT USE INTERCOM"))))

(fn ConstructionScript
  (|CallParentFunction))

(fn IsInteractable
  (return (Variables|Default|GetInteractable)))