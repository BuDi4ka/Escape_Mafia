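; BP_Light is a switchable spotlight item for Room1 that also controls plane meshes on two linked window actors.
; ToggleLight flips IsOn and applies it to the SpotLight and the Plane on WindowDick and WindowDonny.
; The WindowDonny update is nested inside the WindowDick validity check, so it only runs when WindowDick is valid.
; The construction script sets the spotlight's initial visibility from IsOn but leaves the window planes untouched.
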(event EventToggleLight
  (bind _window_donny (Variables|Default|GetWindow%20Donny))
  (bind _window_dick_ (Variables|Default|GetWindow%20Dick%20))
  (bind _plane (Variables|/Game/Items/Items_For_Dick/Room1/BP_Window_Dick.BP_Window_Dick_C|GetPlane _window_dick_))
  (bind _plane_2 (Variables|/Game/Items/Items_For_Donny/Room1/BP_Window_Donny.BP_Window_Donny_C|GetPlane _window_donny))
  (bind _output_get (Variables|Default|SetisOn? (not (Variables|Default|GetisOn?))))
  (Rendering|SetVisibility (Variables|Default|GetSpotLight) _output_get false)
  (if (Variables|Default|GetisOn?)
    (Utilities|IsValid _window_dick_
      (:Is%20Valid
        (Rendering|SetVisibility _plane true false)
        (Utilities|IsValid _window_donny
          (:Is%20Valid
            (Rendering|SetVisibility _plane_2 true false)))))
    (else
      (Utilities|IsValid _window_dick_
        (:Is%20Valid
          (Rendering|SetVisibility _plane false false)
          (Utilities|IsValid _window_donny
            (:Is%20Valid
              (Rendering|SetVisibility _plane_2 false false))))))))

(fn ConstructionScript
  (|CallParentFunction)
  (Rendering|SetVisibility (Variables|Default|GetSpotLight) (Variables|Default|GetisOn?) false))