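; BP_WaterDropDick is a Room 1 item Blueprint that animates a falling water drop using a plane component.
; A timeline's Dropping track drives the plane's relative Z downward, but nothing in this file starts that timeline.
; On finish it sets WaterDropped and calls Replay, which immediately clears the flag, hides the plane and restores it to the ReplayPosition transform.
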(fn ConstructionScript)

(fn Replay
  (Rendering|SetVisibility (Variables|Default|GetPlane) false false)
  (Transformation|SetWorldTransform (Variables|Default|GetPlane) (Variables|Default|GetReplay%20Position) false false)
  (Variables|Default|SetbWaterDropped false))