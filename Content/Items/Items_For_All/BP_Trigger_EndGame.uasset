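; End-game trigger that finishes the level when a BP_Character overlaps its box, for two local players.
; The overlap fades both cameras out, then runs nested loops that remove widgets, override WBP_Timer, clear ignored input and switch off BP_Light actors cached at BeginPlay.
; Inside the innermost loop, a delay precedes the completion sound, game pause and one of three endings chosen by evidence flags (none, Dick, Donny) not set here.
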(event OnComponentBeginOverlap(Box)
  (params (OverlappedComponent :type Primitive%20Component%20Object%20Reference) (OtherActor :type Actor%20Object%20Reference) (OtherComp :type Primitive%20Component%20Object%20Reference) (OtherBodyIndex :type Integer) (bFromSweep :type Boolean) (SweepResult :type Hit%20Result%20Structure%20%28by%20ref%29))
  (bind _returnvalue (Game|GetPlayerController 1))
  (bind _returnvalue_2 (Game|GetPlayerController 0))
  (Utilities|Casting|CastToBP_Character OtherActor)
  (CameraFades|StartCameraFade :self (Variables|/Script/Engine.PlayerController|GetPlayerCameraManager (Game|GetPlayerController 0)) :ToAlpha 1.0 :Duration 1.0 :bHoldWhenFinished true)
  (CameraFades|StartCameraFade :self (Variables|/Script/Engine.PlayerController|GetPlayerCameraManager (Game|GetPlayerController 1)) :ToAlpha 1.0 :Duration 1.0 :bHoldWhenFinished true)
  (bind _foundwidgets (Widget|GetAllWidgetsOfClass "/Script/UMG.UserWidget" false))
  (for _array_element _foundwidgets
    (Widget|RemovefromParent _array_element)
    (bind _foundwidgets_2 (Widget|GetAllWidgetsOfClass "/Game/UI/WBP/WBP_Timer.WBP_Timer_C" false))
    (for _array_element_2 _foundwidgets_2
      (bind _aswbp_timer (Utilities|Casting|CastToWBP_Timer _array_element_2))
      (Variables|/Game/UI/WBP/WBP_Timer.WBP_Timer_C|SetTimer _aswbp_timer 12323.0)
      (Input|SetIgnoreLookInput _returnvalue_2 false)
      (Input|SetIgnoreMoveInput _returnvalue_2 false)
      (Input|SetIgnoreLookInput _returnvalue false)
      (Input|SetIgnoreMoveInput _returnvalue false)
      (for _array_element_3 (Variables|Default|GetLight)
        ;[1 1 1] Play Music of Level Completion
        (Variables|/Game/Items/Items_For_All/Room1/BP_Light.BP_Light_C|SetisOn? _array_element_3 false)
        (Utilities|FlowControl|Delay 1.5)
        (Audio|PlaySound2D "/Game/Audio/SFX/LevelCompletion/level_complete_idea.level_complete_idea" 1.0 1.0 0.0 0 0)
        (Game|SetGamePaused true)
        (if (Variables|Default|GetNoEvidence?)
          (bind _returnvalue_3 (UserInterface|CreateWidget "/Game/UI/EndGameStates/WBP_EndGame_NoEvidence.WBP_EndGame_NoEvidence_C"))
          (UserInterface|Viewport|AddtoViewport _returnvalue_3 0)
          (elif (Variables|Default|GetDickEvidence?)
            (bind _returnvalue_4 (UserInterface|CreateWidget "/Game/UI/EndGameStates/WBP_EndGame_DickEvidence.WBP_EndGame_DickEvidence_C"))
            (UserInterface|Viewport|AddtoViewport _returnvalue_4 0)
            (elif (Variables|Default|GetDonnyEvidence?)
              (bind _returnvalue_5 (UserInterface|CreateWidget "/Game/UI/EndGameStates/WBP_EndGame_DonnyEvidence.WBP_EndGame_DonnyEvidence_C"))
              (UserInterface|Viewport|AddtoViewport _returnvalue_5 0))))))))

(event EventBeginPlay
  (Utilities|FlowControl|Delay 0.2)
  (bind _outactors (Actor|GetAllActorsOfClasswithTag "/Game/Items/Items_For_All/Room1/BP_Light.BP_Light_C" "light"))
  (Variables|Default|SetLight _outactors))

(event EventTick
  (params (DeltaSeconds :type Float%20%28single-precision%29)))

(fn ConstructionScript)