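; Interactable intercom (Dick's) that acts as a one-shot step in a chained intercom sequence.
; On BeginPlay it caches the BP_Intercom_Donny actor tagged "donnyintercom".
; When used while CanIntercom is set, it spawns a BP_Book_ForIntercom at a hardcoded location, enables Donny's intercom and disables itself.
; Otherwise it only prints a debug message, and IsInteractable reports the separate Interactable flag.
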(event EventBeginPlay
  (bind _outactors (Actor|GetAllActorsOfClasswithTag "/Game/Items/Items_For_All/BP_Intercom_Donny.BP_Intercom_Donny_C" "donnyintercom"))
  (for _array_element _outactors
    (Variables|Default|SetIntercom%20Donny _array_element)))

(event EventOnIntercom
  (params (IntercomPlayer :type Character%20Object%20Reference))
  (if (Variables|Default|GetcanIntercom)
    (Game|SpawnActorfromClass "/Game/Items/Items_For_Intercom/Room1/BP_Book_ForIntercom.BP_Book_ForIntercom_C" (Math|Transform|MakeTransform "900.000000,237.000000,30.000000" "0, 0, 0" "1.000000,1.000000,1.000000") "Undefined" "MultiplyWithRoot" 0 0)
    (Development|PrintString "Intercom Dick Interacted" true true "(R=0.369792,G=0.000000,B=0.030108,A=1.000000)")
    (Variables|/Game/Items/Items_For_All/BP_Intercom_Donny.BP_Intercom_Donny_C|SetcanIntercom (Variables|Default|GetIntercom%20Donny) true)
    (Variables|Default|SetcanIntercom false)
    (else
      (Development|PrintString "CAN NOT BE USED"))))

(fn ConstructionScript
  (|CallParentFunction))

(fn IsInteractable
  (return (Variables|Default|GetInteractable)))