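; BP_Item is an item actor that shows a widget as an interact prompt when something enters its sphere.
; If Interactable is set, sphere begin and end overlaps toggle IsPrompt and the widget's visibility, with no check on which actor overlaps.
; Tick rotates the widget every frame to face the player camera.
; IsInteractable exposes the Interactable flag, and the file holds no interaction logic itself.
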(event OnComponentBeginOverlap(Sphere)
  (params (OverlappedComponent :type Primitive%20Component%20Object%20Reference) (OtherActor :type Actor%20Object%20Reference) (OtherComp :type Primitive%20Component%20Object%20Reference) (OtherBodyIndex :type Integer) (bFromSweep :type Boolean) (SweepResult :type Hit%20Result%20Structure%20%28by%20ref%29))
  ;[1 1 1] Spawn/Destroy Interact Prompts
  (if (Variables|Default|GetInteractable)
    (Variables|Default|SetisPrompt true)
    (Rendering|SetVisibility (Variables|Default|GetWidget) true false)))

(event OnComponentEndOverlap(Sphere)
  (params (OverlappedComponent :type Primitive%20Component%20Object%20Reference) (OtherActor :type Actor%20Object%20Reference) (OtherComp :type Primitive%20Component%20Object%20Reference) (OtherBodyIndex :type Integer))
  ;[1 1 1] Spawn/Destroy Interact Prompts
  (if (Variables|Default|GetInteractable)
    (Variables|Default|SetisPrompt false)
    (Rendering|SetVisibility (Variables|Default|GetWidget) false false)))

(event EventTick
  (params (DeltaSeconds :type Float%20%28single-precision%29))
  (bind _widget (Variables|Default|GetWidget))
  ;[1 1 1] Turn Widget toward Player
  (Transformation|SetWorldRotation _widget (Math|Rotator|FindLookatRotation (Transformation|GetWorldLocation _widget) (Camera|GetCameraLocation (Game|GetPlayerCameraManager (Variables|Default|GetPlayer%20Index)))) false false))

(fn ConstructionScript)

(fn IsInteractable
  (return (Variables|Default|GetInteractable)))