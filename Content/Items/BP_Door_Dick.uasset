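; BP_Door_Dick is an interactable door that opens only for a BP_Dick player holding the Room 1 key.
; BeginPlay caches the player character as BP_Dick, and OnInteract checks its HasKeyRoom1 flag.
; With the key, a DoOnce prints an open message and snaps the Cube to a rotated position; otherwise a missing-key message prints.
; IsInteractable always returns true.
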(event EventOnInteract
  (params (InteractingPlayer :type Character%20Object%20Reference))
  (if (Variables|/Game/Character/Dick/BP_Dick.BP_Dick_C|GethasKeyRoom1? (Variables|Default|GetBP%20Dick))
    (Utilities|FlowControl|DoOnce false
      (:Completed
        (Development|PrintString "DICK DOOR IS OPEN" true true "(R=0.054720,G=0.019952,B=0.406250,A=1.000000)" 1e+01)
        (Transformation|SetRelativeRotation (Variables|Default|GetCube) "0.000000,90.000000,0.000000" false false)))
    (else
      (Development|PrintString "YOU DONT HAVE A KEY" true true "(R=1.000000,G=0.000000,B=0.026838,A=1.000000)" 1e+01))))

(event EventBeginPlay
  (bind _asbp_dick (Utilities|Casting|CastToBP_Dick (Game|GetPlayerCharacter 0)))
  (Variables|Default|SetBP%20Dick _asbp_dick))

(fn ConstructionScript
  (|CallParentFunction))

(fn IsInteractable
  (return true))