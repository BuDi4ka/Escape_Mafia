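; BP_Axe2Donny is an axe item for Donny in Room1 that shakes while its BP_Axe2Dick counterpart has not been interacted with.
; On BeginPlay it looks up the BP_Axe2Dick actors and starts a fast looping timer.
; Each tick of that timer checks the first actor's Interacted flag and, while false, restarts a timeline that drives the Axe2 component's relative roll.
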(event Custom|Check
  (if (not (Variables|/Game/Items/Items_For_Dick/Room1/BP_Axe2Dick.BP_Axe2Dick_C|GetInteracted (Utilities|Array|Get(acopy) (stale EventBeginPlay _outactors))))
    (bind _shake (Timeline|ShakeTimeline PlayFromStart)
      (:Update
        (Transformation|SetRelativeRotation (Variables|Default|GetAxe2) (Math|Rotator|MakeRotator (* _shake 5.0) 0.0 0.0) false false)))))

(event EventBeginPlay
  (bind _outactors (Actor|GetAllActorsOfClass "/Game/Items/Items_For_Dick/Room1/BP_Axe2Dick.BP_Axe2Dick_C"))
  (Utilities|Time|SetTimerbyEvent (delegate Custom|Check) 0.1 true))

(fn ConstructionScript
  (|CallParentFunction))