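; BP_CupboardDoorLeftDonny is a left cupboard door in Donny's Room1 that mirrors the state of its counterpart, BP_CupboardDoorLeftDick.
; BeginPlay finds the Dick door actors and starts a fast looping timer that polls the first one's Interacted flag.
; The flag plays or reverses the OpenClose timeline, which swings the Door component in relative yaw.
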(event Custom|Check
  (if (Variables|/Game/Items/Items_For_Dick/Room1/BP_CupboardDoorLeftDick.BP_CupboardDoorLeftDick_C|GetInteracted (Utilities|Array|Get(acopy) (stale EventBeginPlay _outactors)))
    (bind _anim (Timeline|Open/Close Play)
      (:Update
        (Transformation|SetRelativeRotation (Variables|Default|GetDoor) (Math|Rotator|MakeRotator 0.0 0.0 (* _anim -9e+01)) false false)))
    (else
      (Timeline|Open/Close Reverse))))

(event EventBeginPlay
  (bind _outactors (Actor|GetAllActorsOfClass "/Game/Items/Items_For_Dick/Room1/BP_CupboardDoorLeftDick.BP_CupboardDoorLeftDick_C"))
  (Utilities|Time|SetTimerbyEvent (delegate Custom|Check) 0.1 true))

(fn ConstructionScript
  (|CallParentFunction))