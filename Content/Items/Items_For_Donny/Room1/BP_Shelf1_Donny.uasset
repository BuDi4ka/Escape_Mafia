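; BP_Shelf1_Donny is a Room1 shelf for Donny that mirrors the open state of its counterpart, BP_Shelf1_Dick.
; BeginPlay finds the Dick shelf actors in the level, and Tick polls the first one's ShelfOpen flag.
; The flag plays or reverses a timeline that slides the Cube along its relative X axis to open or close the shelf.
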(event EventBeginPlay
  (bind _outactors (Actor|GetAllActorsOfClass "/Game/Items/Items_For_Dick/Room1/BP_Shelf1_Dick.BP_Shelf1_Dick_C")))

(event EventTick
  (params (DeltaSeconds :type Float%20%28single-precision%29))
  (if (== (Variables|/Game/Items/Items_For_Dick/Room1/BP_Shelf1_Dick.BP_Shelf1_Dick_C|GetShelfOpen (Utilities|Array|Get(acopy) (stale EventBeginPlay _outactors))) true)
    (bind _open_close_shelf (Timeline|Shelf%201Donny Play)
      (:Update
        (Transformation|SetRelativeLocation (Variables|Default|GetCube) (Math|Vector|MakeVector (* _open_close_shelf 5e+01) 0.0 0.0) false false)))
    (else
      (Timeline|Shelf%201Donny Reverse))))

(fn ConstructionScript
  (|CallParentFunction))