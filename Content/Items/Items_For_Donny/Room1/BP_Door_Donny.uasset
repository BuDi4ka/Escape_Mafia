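; BP_Door_Donny is an interactable door that swings open once and also opens its counterpart BP_Door_Dick actors tagged "door", found at BeginPlay.
; OnInteract plays a timeline that rotates the Cube's yaw, calls OpenDoor on each counterpart every update, and disables interaction.
; Sphere overlaps toggle an outline overlay, while a fast looping timer shows the prompt widget.
; Tick turns that widget toward player 1's camera.
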(event OnComponentBeginOverlap(Sphere)
  (params (OverlappedComponent :type Primitive%20Component%20Object%20Reference) (OtherActor :type Actor%20Object%20Reference) (OtherComp :type Primitive%20Component%20Object%20Reference) (OtherBodyIndex :type Integer) (bFromSweep :type Boolean) (SweepResult :type Hit%20Result%20Structure%20%28by%20ref%29))
  (if (Variables|Default|GetInteractable)
    (Rendering|Material|SetOverlayMaterial (Variables|Default|GetCube) "/Game/Assets/Materials/M_Outline.M_Outline" :!class /Script/Engine.MeshComponent)))

(event OnComponentEndOverlap(Sphere)
  (params (OverlappedComponent :type Primitive%20Component%20Object%20Reference) (OtherActor :type Actor%20Object%20Reference) (OtherComp :type Primitive%20Component%20Object%20Reference) (OtherBodyIndex :type Integer))
  (Rendering|Material|SetOverlayMaterial (Variables|Default|GetCube) 0 :!class /Script/Engine.MeshComponent))

(event Custom|CheckWidget
  (if (and (Variables|Default|GetInteractable) (Variables|Default|GetisPrompt))
    (Rendering|SetVisibility (Variables|Default|GetWidget) true false)
    (Rendering|Material|SetOverlayMaterial (Variables|Default|GetCube) "/Game/Assets/Materials/M_Outline.M_Outline" :!class /Script/Engine.MeshComponent)))

(event EventTick
  (params (DeltaSeconds :type Float%20%28single-precision%29))
  (bind _widget (Variables|Default|GetWidget))
  (Transformation|SetWorldRotation _widget (Math|Rotator|FindLookatRotation (Transformation|GetWorldLocation _widget) (Camera|GetCameraLocation (Game|GetPlayerCameraManager 1))) false false))

(event EventOnInteract
  (params (InteractingPlayer :type Character%20Object%20Reference) (Player%20Index :type Integer))
  (Utilities|FlowControl|DoOnce false
    (:Completed
      (bind _doorfloat (Timeline|Timeline Play)
        (:Update
          (Transformation|SetRelativeRotation (Variables|Default|GetCube) (Math|Rotator|MakeRotator 0.0 0.0 (Math|Float|Lerp 1e+01 9e+01 _doorfloat)) false false)
          (for _array_element (Variables|Default|GetDickDoor)
            (Default|OpenDoor _array_element)
            (Variables|Default|SetInteractable false)
            (Rendering|SetVisibility (Variables|Default|GetWidget) false false)
            (Rendering|Material|SetOverlayMaterial (Variables|Default|GetCube) 0 :!class /Script/Engine.MeshComponent)))))))

(event EventBeginPlay
  (bind _outactors (Actor|GetAllActorsOfClasswithTag "/Game/Items/Items_For_Dick/Room1/BP_Door_Dick.BP_Door_Dick_C" "door"))
  (Variables|Default|SetDickDoor _outactors)
  (Utilities|Time|SetTimerbyEvent (delegate Custom|CheckWidget) 0.01 true))

(fn ConstructionScript
  (|CallParentFunction))