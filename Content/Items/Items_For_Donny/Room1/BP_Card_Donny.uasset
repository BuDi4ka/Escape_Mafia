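; BP_Card_Donny is an interactable card item in Donny's Room1 that can be picked up.
; Interacting sets CardDestroyed on BP_Donny, fetched as player character index 1, then destroys the card.
; Sphere overlap adds an outline overlay material to the cylinder while interactable and clears it on exit.
; A 0.01-second looping timer also shows the prompt widget and outline whenever Interactable and IsPrompt are true.
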(event OnComponentBeginOverlap(Sphere)
  (params (OverlappedComponent :type Primitive%20Component%20Object%20Reference) (OtherActor :type Actor%20Object%20Reference) (OtherComp :type Primitive%20Component%20Object%20Reference) (OtherBodyIndex :type Integer) (bFromSweep :type Boolean) (SweepResult :type Hit%20Result%20Structure%20%28by%20ref%29))
  (if (Variables|Default|GetInteractable)
    (Rendering|Material|SetOverlayMaterial (Variables|Default|GetCylinder) "/Game/Assets/Materials/M_Outline.M_Outline" :!class /Script/Engine.MeshComponent)))

(event OnComponentEndOverlap(Sphere)
  (params (OverlappedComponent :type Primitive%20Component%20Object%20Reference) (OtherActor :type Actor%20Object%20Reference) (OtherComp :type Primitive%20Component%20Object%20Reference) (OtherBodyIndex :type Integer))
  (Rendering|Material|SetOverlayMaterial (Variables|Default|GetCylinder) 0 :!class /Script/Engine.MeshComponent))

(event Custom|CheckWidget
  (if (and (Variables|Default|GetInteractable) (Variables|Default|GetisPrompt))
    (Rendering|SetVisibility (Variables|Default|GetWidget) true false)
    (Rendering|Material|SetOverlayMaterial (Variables|Default|GetCylinder) "/Game/Assets/Materials/M_Outline.M_Outline" :!class /Script/Engine.MeshComponent)))

(event EventOnInteract
  (params (InteractingPlayer :type Character%20Object%20Reference) (Player%20Index :type Integer))
  (bind _asbp_donny (Utilities|Casting|CastToBP_Donny (Game|GetPlayerCharacter 1)))
  ;[1 1 1] on interact
  (Variables|/Game/Character/Donny/BP_Donny.BP_Donny_C|SetCardDestroyed _asbp_donny true)
  (Actor|DestroyActor))

(event EventBeginPlay
  (Utilities|Time|SetTimerbyEvent (delegate Custom|CheckWidget) 0.01 true))

(fn ConstructionScript
  (|CallParentFunction))