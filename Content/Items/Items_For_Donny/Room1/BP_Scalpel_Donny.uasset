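; Scalpel item for Donny that, when used, allows the player to finish the level and unlocks the doors.
; A fast looping timer shows the prompt widget while player 1 overlaps, and sphere overlaps toggle the outline overlay material when Donny isn't jumping.
; A one-time interaction hides the scalpel, plays sounds, rotates the tagged Dick and Donny doors found at BeginPlay, and makes Donny's doors interactable.
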(event OnComponentBeginOverlap(Sphere)
  (params (OverlappedComponent :type Primitive%20Component%20Object%20Reference) (OtherActor :type Actor%20Object%20Reference) (OtherComp :type Primitive%20Component%20Object%20Reference) (OtherBodyIndex :type Integer) (bFromSweep :type Boolean) (SweepResult :type Hit%20Result%20Structure%20%28by%20ref%29))
  (bind _asbp_donny (Utilities|Casting|CastToBP_Donny OtherActor))
  (if (not (Variables|/Game/Character/Donny/BP_Donny.BP_Donny_C|GetisJumping _asbp_donny))
    (if (Variables|Default|GetInteractable)
      (Rendering|Material|SetOverlayMaterial (Variables|Default|GetCylinder) "/Game/Assets/Materials/M_Outline.M_Outline" :!class /Script/Engine.MeshComponent))))

(event OnComponentEndOverlap(Sphere)
  (params (OverlappedComponent :type Primitive%20Component%20Object%20Reference) (OtherActor :type Actor%20Object%20Reference) (OtherComp :type Primitive%20Component%20Object%20Reference) (OtherBodyIndex :type Integer))
  (bind _asbp_donny (Utilities|Casting|CastToBP_Donny OtherActor))
  (if (not (Variables|/Game/Character/Donny/BP_Donny.BP_Donny_C|GetisJumping _asbp_donny))
    (Rendering|Material|SetOverlayMaterial (Variables|Default|GetCylinder) 0 :!class /Script/Engine.MeshComponent)))

(event Custom|CheckWidget
  (bind _widget (Variables|Default|GetWidget))
  (if (Math|Boolean|ANDBoolean (Variables|Default|GetInteractable) (Variables|Default|GetisPrompt) (Collision|IsOverlappingActor (Game|Player|GetPlayerPawn 1) :!class /Script/Engine.Actor))
    (Rendering|SetVisibility _widget true false)
    (Rendering|Material|SetOverlayMaterial (Variables|Default|GetCylinder) "/Game/Assets/Materials/M_Outline.M_Outline" :!class /Script/Engine.MeshComponent)
    (else
      (Rendering|SetVisibility _widget false false))))

(event EventOnInteract
  (params (InteractingPlayer :type Character%20Object%20Reference) (Player%20Index :type Integer))
  (Utilities|FlowControl|DoOnce false
    (:Completed
      (Audio|PlaySound2D "/Game/Audio/SFX/Interaction/interaction_sfx_v1.interaction_sfx_v1" 1.0 1.0 0.0 0 0)
      (bind _asbp_donny (Utilities|Casting|CastToBP_Donny (Game|GetPlayerCharacter 1)))
      ;[1 1 1] On Interact
      (Variables|/Game/Character/Donny/BP_Donny.BP_Donny_C|SetcanFinishLevel? _asbp_donny true)
      (Rendering|SetVisibility (Variables|Default|GetCylinder) false false)
      (Variables|Default|SetInteractable false)
      (Variables|Default|SetisPrompt false)
      (Rendering|SetVisibility (Variables|Default|GetWidget) false false)
      (Audio|PlaySound2D "/Game/Audio/SFX/big_door_unlock_sfx.big_door_unlock_sfx" 1.0 1.0 0.0 0 0)
      (for _array_element (Variables|Default|GetDickDoor)
        (Transformation|SetRelativeRotation (Variables|/Game/Items/Items_For_Dick/Room1/BP_Door_Dick.BP_Door_Dick_C|GetCube _array_element) "0.000000,10.000000,0.000000" false false)
        (for _array_element_2 (Variables|Default|GetDonnyDoor)
          (Transformation|SetRelativeRotation (Variables|/Game/Items/Items_For_Donny/Room1/BP_Door_Donny.BP_Door_Donny_C|GetCube _array_element_2) "0.000000,10.000000,0.000000" false false)
          (Variables|/Game/Items/BP_Item.BP_Item_C|SetInteractable _array_element_2 true))))))

(event EventBeginPlay
  (Utilities|Time|SetTimerbyEvent (delegate Custom|CheckWidget) 0.01 true)
  (bind _outactors (Actor|GetAllActorsOfClasswithTag "/Game/Items/Items_For_Dick/Room1/BP_Door_Dick.BP_Door_Dick_C" "door"))
  (Variables|Default|SetDickDoor _outactors)
  (bind _outactors_2 (Actor|GetAllActorsOfClasswithTag "/Game/Items/Items_For_Donny/Room1/BP_Door_Donny.BP_Door_Donny_C" "door"))
  (Variables|Default|SetDonnyDoor _outactors_2))

(fn ConstructionScript
  (|CallParentFunction))