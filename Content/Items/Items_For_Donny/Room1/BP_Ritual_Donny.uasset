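; BP_Ritual_Donny is an interactable ritual item that toggles the WBP_Ritual widget on the second local player's screen.
; Each interaction flip-flops between showing the widget with movement and look locked for player controller 1, and removing it.
; Input mode and cursor changes target player controller 0.
; Leaving the Box also closes a valid widget, while the Sphere toggles the Cylinder's outline overlay, shown only when interactable.
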(event OnComponentEndOverlap(Box)
  (params (OverlappedComponent :type Primitive%20Component%20Object%20Reference) (OtherActor :type Actor%20Object%20Reference) (OtherComp :type Primitive%20Component%20Object%20Reference) (OtherBodyIndex :type Integer))
  (bind _returnvalue (Game|GetPlayerController 1))
  (bind _returnvalue_2 (Game|GetPlayerController 0))
  (Utilities|IsValid (stale EventOnInteract _returnvalue_5)
    (:Is%20Valid
      (Widget|RemovefromParent (stale EventOnInteract _returnvalue_5))
      (Input|SetInputModeGameOnly _returnvalue_2 false)
      (Variables|/Script/Engine.PlayerController|SetbShowMouseCursor _returnvalue_2 false)
      (Input|SetIgnoreMoveInput _returnvalue false)
      (Input|SetIgnoreLookInput _returnvalue false))))

(event OnComponentBeginOverlap(Sphere)
  (params (OverlappedComponent :type Primitive%20Component%20Object%20Reference) (OtherActor :type Actor%20Object%20Reference) (OtherComp :type Primitive%20Component%20Object%20Reference) (OtherBodyIndex :type Integer) (bFromSweep :type Boolean) (SweepResult :type Hit%20Result%20Structure%20%28by%20ref%29))
  (if (Variables|Default|GetInteractable)
    (Rendering|Material|SetOverlayMaterial (Variables|Default|GetCylinder) "/Game/Assets/Materials/M_Outline.M_Outline" :!class /Script/Engine.MeshComponent)))

(event OnComponentEndOverlap(Sphere)
  (params (OverlappedComponent :type Primitive%20Component%20Object%20Reference) (OtherActor :type Actor%20Object%20Reference) (OtherComp :type Primitive%20Component%20Object%20Reference) (OtherBodyIndex :type Integer))
  (Rendering|Material|SetOverlayMaterial (Variables|Default|GetCylinder) 0 :!class /Script/Engine.MeshComponent))

(event EventOnInteract
  (params (InteractingPlayer :type Character%20Object%20Reference) (Player%20Index :type Integer))
  (bind _returnvalue (Game|GetPlayerController 0))
  (bind _returnvalue_2 (Game|GetPlayerController 1))
  (bind _returnvalue_3 (Game|GetPlayerController 1))
  (bind _returnvalue_4 (Game|GetPlayerController 0))
  ;[1 1 1] On Interact
  (Utilities|FlowControl|FlipFlop
    (:A
      (bind _returnvalue_5 (UserInterface|CreateWidget "/Game/UI/WBP/WBP_Ritual.WBP_Ritual_C" (Game|GetPlayerController 1)))
      (UserInterface|Viewport|AddtoPlayerScreen _returnvalue_5)
      (Input|SetInputModeGameandUI _returnvalue _returnvalue_5 "DoNotLock" true false)
      (Variables|/Script/Engine.PlayerController|SetbShowMouseCursor _returnvalue true)
      (Input|SetIgnoreMoveInput _returnvalue_2 true)
      (Input|SetIgnoreLookInput _returnvalue_2 true))
    (:B
      (Widget|RemovefromParent _returnvalue_5)
      (Input|SetInputModeGameOnly _returnvalue_4 false)
      (Variables|/Script/Engine.PlayerController|SetbShowMouseCursor _returnvalue_4 false)
      (Input|SetIgnoreMoveInput _returnvalue_3 false)
      (Input|SetIgnoreLookInput _returnvalue_3 false))))

(fn ConstructionScript
  (|CallParentFunction))