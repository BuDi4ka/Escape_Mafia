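; BP_Axe1Donny is an axe item in Donny's Room1 set that shakes until its BP_Axe1Dick counterpart has been interacted with.
; BeginPlay looks up the BP_Axe1Dick actors, and Tick polls the first one's Interacted flag.
; While the flag is false, Tick restarts the ShakeAxe timeline every frame, whose ShakeAnim track drives the axe's relative roll.
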(event EventBeginPlay
  (bind _outactors (Actor|GetAllActorsOfClass "/Game/Items/Items_For_Dick/Room1/BP_Axe1Dick.BP_Axe1Dick_C")))

(event EventTick
  (params (DeltaSeconds :type Float%20%28single-precision%29))
  (if (not (Variables|/Game/Items/Items_For_Dick/Room1/BP_Axe1Dick.BP_Axe1Dick_C|GetInteracted (Utilities|Array|Get(acopy) (stale EventBeginPlay _outactors))))
    (bind _shakeanim (Timeline|ShakeAxe PlayFromStart)
      (:Update
        (Transformation|SetRelativeRotation (Variables|Default|GetAxe) (Math|Rotator|MakeRotator (* _shakeanim 1.0) 0.0 0.0) false false)))))

(fn ConstructionScript
  (|CallParentFunction))