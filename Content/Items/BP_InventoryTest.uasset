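; BP_InventoryTest is a test pickup item for the inventory system.
; Its Construction Script uses the item ID enum name as the row name in DT_ItemInfo to fill SItemInfo.
; On OnInteract, if CanPickUp is set, it passes that struct to the indexed player's character through PickupMessage, prints a pickup message and destroys itself.
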(event EventOnInteract
  (params (InteractingPlayer :type Character%20Object%20Reference) (Player%20Index :type Integer))
  (bind _s_iteminfo (Variables|Default|GetS_ItemInfo))
  (if (Variables|Default|GetcanPickUp)
    (Class|BPIPickupItem|Pickup(Message) (Game|GetPlayerCharacter Player%20Index) _s_iteminfo)
    (Development|PrintString (Utilities|String|Append "Player " (Utilities|String|ToString(Integer) Player%20Index) " Has Picked Up " (Utilities|String|ToString(Text) (.ItemName (Utilities|Struct|BreakS_ItemInfo _s_iteminfo)))))
    (Actor|DestroyActor)))

(fn ConstructionScript
  (bind _returnvalue (Utilities|GetDataTableRow "/Game/Character/Inventory/DT_ItemInfo.DT_ItemInfo" (Utilities|String|StringToName (Utilities|String|EnumtoString (.ItemID (Utilities|Struct|BreakS_ItemInfo (Variables|Default|GetS_ItemInfo))))))
    (:then
      (Variables|Default|SetS_ItemInfo _returnvalue))))