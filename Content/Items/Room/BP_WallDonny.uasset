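; BP_WallDonny is a wall that Donny, the character of player index 1, can pass through while jumping if a light is off.
; After a short BeginPlay delay it caches Donny and starts a fast looping timer.
; Each tick of that timer disables the Cube's collision if Donny is jumping and any "light"-tagged BP_Light is off, and restores collision whenever Donny is not jumping.
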(event Custom|CheckJumping
  (if (Variables|/Game/Character/Donny/BP_Donny.BP_Donny_C|GetisJumping (Variables|Default|GetDonny))
    (bind _outactors (Actor|GetAllActorsOfClasswithTag "/Game/Items/Items_For_All/Room1/BP_Light.BP_Light_C" "light"))
    (for _array_element _outactors
      (if (not (Variables|/Game/Items/Items_For_All/Room1/BP_Light.BP_Light_C|GetisOn? _array_element))
        (Collision|SetCollisionEnabled (Variables|Default|GetCube) "NoCollision")))
    (else
      (Collision|SetCollisionEnabled (Variables|Default|GetCube) "QueryAndPhysics"))))

(event EventBeginPlay
  (Utilities|FlowControl|Delay 0.1)
  (bind _asbp_donny (Utilities|Casting|CastToBP_Donny (Game|GetPlayerCharacter 1)))
  (Variables|Default|SetDonny _asbp_donny)
  (Utilities|Time|SetTimerbyEvent (delegate Custom|CheckJumping) 0.01 true))

(fn ConstructionScript)