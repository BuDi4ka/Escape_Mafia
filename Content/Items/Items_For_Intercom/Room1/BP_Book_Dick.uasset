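; BP_Book_Dick is an interactable book pickup in Room1 of the intercom items that unlocks Dick's pneumatic actors.
; On BeginPlay it caches the tagged Dick and Donny pneumatic actors.
; On interact it destroys itself, prints a pickup message, makes Dick's pneumatics interactable and resets both sets' cube materials to BasicAsset01.
; Donny's pneumatics only change material, inside the Dick loop, and no inventory write occurs despite the graph comment.
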(event EventBeginPlay
  (bind _outactors (Actor|GetAllActorsOfClasswithTag "/Game/Items/Items_For_Dick/Room1/BP_Pneumatic_Dick.BP_Pneumatic_Dick_C" "dickpneumatic"))
  (Variables|Default|Setdick_pneumatic _outactors)
  (bind _outactors_2 (Actor|GetAllActorsOfClasswithTag "/Game/Items/Items_For_Donny/Room1/BP_Pneumatic_Donny.BP_Pneumatic_Donny_C" "donnypneumatic"))
  (Variables|Default|Setdonny_pneumatic _outactors_2))

(event EventOnInteract
  (params (InteractingPlayer :type Character%20Object%20Reference))
  ;[1 1 1] add to Dick Inventory
  (Actor|DestroyActor)
  (Development|PrintString "BOOK PICKED UP" true true "(R=1.000000,G=0.805564,B=0.000000,A=1.000000)" 3.0)
  (for _array_element (Variables|Default|Getdick_pneumatic)
    (Variables|/Game/Items/Items_For_Dick/Room1/BP_Pneumatic_Dick.BP_Pneumatic_Dick_C|SetInteractable _array_element true)
    (Rendering|Material|SetMaterial (Variables|/Game/Items/Items_For_Dick/Room1/BP_Pneumatic_Dick.BP_Pneumatic_Dick_C|GetCube _array_element) 0 "/Engine/MapTemplates/Materials/BasicAsset01.BasicAsset01")
    (for _array_element_2 (Variables|Default|Getdonny_pneumatic)
      (Rendering|Material|SetMaterial (Variables|/Game/Items/Items_For_Donny/Room1/BP_Pneumatic_Donny.BP_Pneumatic_Donny_C|GetCube _array_element_2) 0 "/Engine/MapTemplates/Materials/BasicAsset01.BasicAsset01"))))

(fn ConstructionScript
  (|CallParentFunction))

(fn IsInteractable
  (return (Variables|Default|GetInteractable)))