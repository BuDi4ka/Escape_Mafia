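; Book pickup for the Room 1 intercom items, always reporting itself as interactable.
; On BeginPlay it finds the Donny and Dick intercom actors by class and tag and caches them.
; Interacting destroys the book, shows a pickup debug message and hides the Dick intercom's Cube; the Donny reference goes unused.
; The intercom event only destroys the actor, and neither event makes an actual inventory call despite the graph comments.
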(event EventBeginPlay
  (Utilities|FlowControl|Sequence
    (:then_0
      (bind _outactors (Actor|GetAllActorsOfClasswithTag "/Game/Items/Items_For_All/Room1/BP_Intercom_Donny.BP_Intercom_Donny_C" "donny intercom"))
      (for _array_element _outactors
        (Variables|Default|SetIntercomDonny _array_element)))
    (:then_1
      (bind _outactors_2 (Actor|GetAllActorsOfClasswithTag "/Game/Items/Items_For_All/Room1/BP_Intercom_Dick.BP_Intercom_Dick_C" "dick intercom"))
      (for _array_element_2 _outactors_2
        (Variables|Default|SetIntercomDick _array_element_2)))))

(event EventOnInteract
  (params (InteractingPlayer :type Character%20Object%20Reference))
  ;[1 1 1] Add to Player Inventory
  (Actor|DestroyActor)
  (Development|PrintString "BOOK PICKED UP" true true "(R=1.000000,G=0.805564,B=0.000000,A=1.000000)" 3.0)
  (Rendering|SetVisibility (Variables|/Game/Items/Items_For_All/Room1/BP_Intercom_Dick.BP_Intercom_Dick_C|GetCube (Variables|Default|GetIntercomDick)) false false))

(event EventOnIntercom
  (params (IntercomPlayer :type Character%20Object%20Reference))
  ;[1 1 1] Delete from Player Inventory
  (Actor|DestroyActor))

(fn ConstructionScript
  (|CallParentFunction))

(fn IsInteractable
  (return true))