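; BP_Dial_Dick is an interactable dial prop for Room1 that opens the WBP_Dial screen widget.
; OnInteract uses a FlipFlop to open or close the widget, switching input mode and mouse cursor to match.
; Leaving the Box also closes a valid widget, without resetting the FlipFlop.
; Sphere overlap toggles the Cone's outline when Interactable is set, though IsInteractable always returns false.
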(event OnComponentEndOverlap(Box)
  (params (OverlappedComponent :type Primitive%20Component%20Object%20Reference) (OtherActor :type Actor%20Object%20Reference) (OtherComp :type Primitive%20Component%20Object%20Reference) (OtherBodyIndex :type Integer))
  (bind _returnvalue (Game|GetPlayerController 0))
  (Utilities|IsValid (stale EventOnInteract _returnvalue_3)
    (:Is%20Valid
      (Widget|RemovefromParent (stale EventOnInteract _returnvalue_3))
      (Input|SetInputModeGameOnly _returnvalue false)
      (Variables|/Script/Engine.PlayerController|SetbShowMouseCursor _returnvalue false))))

(event OnComponentBeginOverlap(Sphere)
  (params (OverlappedComponent :type Primitive%20Component%20Object%20Reference) (OtherActor :type Actor%20Object%20Reference) (OtherComp :type Primitive%20Component%20Object%20Reference) (OtherBodyIndex :type Integer) (bFromSweep :type Boolean) (SweepResult :type Hit%20Result%20Structure%20%28by%20ref%29))
  (if (Variables|Default|GetInteractable)
    (Rendering|Material|SetOverlayMaterial (Variables|Default|GetCone) "/Game/Assets/Materials/M_Outline.M_Outline" :!class /Script/Engine.MeshComponent)))

(event OnComponentEndOverlap(Sphere)
  (params (OverlappedComponent :type Primitive%20Component%20Object%20Reference) (OtherActor :type Actor%20Object%20Reference) (OtherComp :type Primitive%20Component%20Object%20Reference) (OtherBodyIndex :type Integer))
  (Rendering|Material|SetOverlayMaterial (Variables|Default|GetCone) 0 :!class /Script/Engine.MeshComponent))

(event EventOnInteract
  (params (InteractingPlayer :type Character%20Object%20Reference) (Player%20Index :type Integer))
  (bind _returnvalue (Game|GetPlayerController 0))
  (bind _returnvalue_2 (Game|GetPlayerController 0))
  ;[1 1 1] On Interact
  (Utilities|FlowControl|FlipFlop
    (:A
      (bind _returnvalue_3 (UserInterface|CreateWidget "/Game/UI/WBP/WBP_Dial.WBP_Dial_C" (Game|GetPlayerController 0)))
      (UserInterface|Viewport|AddtoPlayerScreen _returnvalue_3)
      (Input|SetInputModeGameandUI _returnvalue _returnvalue_3 "DoNotLock" true false)
      (Variables|/Script/Engine.PlayerController|SetbShowMouseCursor _returnvalue true))
    (:B
      (Widget|RemovefromParent _returnvalue_3)
      (Input|SetInputModeGameOnly _returnvalue_2 false)
      (Variables|/Script/Engine.PlayerController|SetbShowMouseCursor _returnvalue_2 false))))

(fn ConstructionScript
  (|CallParentFunction))

(fn IsInteractable
  (return false))