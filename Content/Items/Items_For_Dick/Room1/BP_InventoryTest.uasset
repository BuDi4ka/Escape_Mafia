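; BP_InventoryTest is an interactable pickup item that hands its item data to the interacting player.
; The construction script fills ItemInfo from DT_ItemDataTable, using the ItemID enum name as the row name.
; On interact it sends ItemInfo to that player's character through PickupMessage, prints a debug pickup line and destroys itself.
; IsInteractable always returns true.
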(event EventOnInteract
  (params (PlayerIndex :type Integer))
  (Class|BPIPickup|Pickup(Message) (Game|GetPlayerCharacter PlayerIndex) (Variables|Default|GetItemInfo))
  (Development|PrintString (Utilities|String|Append "Player " (Utilities|String|ToString(Integer) PlayerIndex) " Picked Up " (Utilities|String|ToString(Text) (.ItemName (Utilities|Struct|BreakS_ItemInfo (Variables|Default|GetItemInfo))))))
  (Actor|DestroyActor))

(fn ConstructionScript
  (bind _returnvalue (Utilities|GetDataTableRow "/Game/Items/Inventory/DT_ItemDataTable.DT_ItemDataTable" (Utilities|String|StringToName (Utilities|String|EnumtoString (.ItemID (Utilities|Struct|BreakS_ItemInfo (Variables|Default|GetItemInfo))))))
    (:then
      (Variables|Default|SetItemInfo _returnvalue))))

(fn IsInteractable
  (return true))