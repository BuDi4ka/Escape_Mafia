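; BP_Switch_Dick is an interactable light switch that toggles the lights sharing its LightIndex.
; On BeginPlay it caches every BP_Light actor tagged "light" in an array.
; On interact it loops through that array and calls ToggleLightMessage on each matching light, so one switch can drive several lights.
; It always reports itself as interactable.
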(event EventOnInteract
  (params (InteractingPlayer :type Character%20Object%20Reference) (Player%20Index :type Integer))
  (for _array_element (Variables|Default|GetLightsArray)
    (if (== (Variables|/Game/Items/Items_For_All/Room1/BP_Light.BP_Light_C|GetLightIndex _array_element) (Variables|Default|GetLightIndex))
      (Class|BPILight|ToggleLight(Message) _array_element))))

(event EventBeginPlay
  (bind _outactors (Actor|GetAllActorsOfClasswithTag "/Game/Items/Items_For_All/Room1/BP_Light.BP_Light_C" "light"))
  (for _array_element _outactors
    (Utilities|Array|Add (Variables|Default|GetLightsArray) _array_element)))

(fn ConstructionScript
  (|CallParentFunction))

(fn IsInteractable
  (return true))