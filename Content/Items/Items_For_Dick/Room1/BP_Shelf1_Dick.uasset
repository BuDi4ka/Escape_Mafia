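; Interactable shelf for Dick in Room1 that slides open and closed on alternating interactions via a FlipFlop.
; Each toggle instantly offsets its Cube along world X, along with the optional Evidence actor's cube and every BP_Shelf1_Donny tagged "shelf1donny" found at BeginPlay, mirroring the move on Donny's shelf.
; A fast looping timer shows the prompt widget while Interactable and IsPrompt are true, with no branch to hide it.
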(event Custom|CheckWidget
  (if (and (Variables|Default|GetInteractable) (Variables|Default|GetisPrompt))
    (Rendering|SetVisibility (Variables|Default|GetWidget) true false)))

(event EventBeginPlay
  (Utilities|Time|SetTimerbyEvent (delegate Custom|CheckWidget) 0.01 true)
  (bind _outactors (Actor|GetAllActorsOfClasswithTag "/Game/Items/Items_For_Donny/Room1/BP_Shelf1_Donny.BP_Shelf1_Donny_C" "shelf1donny"))
  (Variables|Default|Setshelf_1_donny _outactors))

(event EventOnInteract
  (params (InteractingPlayer :type Character%20Object%20Reference) (Player%20Index :type Integer))
  (bind _evidence (Variables|Default|GetEvidence))
  ;[1 1 1] On Interact
  (Utilities|FlowControl|FlipFlop
    (:A
      (CallFunction|OpenShelf1Dick)
      (Utilities|IsValid _evidence
        (:Is%20Valid
          (CallFunction|OpenEvidence)
          (CallFunction|OpenShelf1Donny))
        (:Is%20Not%20Valid
          (CallFunction|OpenShelf1Donny))))
    (:B
      (CallFunction|CloseShelf1Dick)
      (Utilities|IsValid _evidence
        (:Is%20Valid
          (CallFunction|CloseEvidence)
          (CallFunction|CloseShelf1Donny))
        (:Is%20Not%20Valid
          (CallFunction|CloseShelf1Donny))))))

(fn ConstructionScript
  (|CallParentFunction))

(fn OpenShelf1Donny
  (for _array_element (Variables|Default|Getshelf_1_donny)
    (Transformation|SetWorldLocation (Variables|/Game/Items/Items_For_Donny/Room1/BP_Shelf1_Donny.BP_Shelf1_Donny_C|GetCube _array_element) (Math|Vector|MakeVector (+ (.x (Transformation|GetWorldLocation (Variables|/Game/Items/Items_For_Donny/Room1/BP_Shelf1_Donny.BP_Shelf1_Donny_C|GetCube _array_element))) 5e+01) (.y (Transformation|GetWorldLocation (Variables|/Game/Items/Items_For_Donny/Room1/BP_Shelf1_Donny.BP_Shelf1_Donny_C|GetCube _array_element))) (.z (Transformation|GetWorldLocation (Variables|/Game/Items/Items_For_Donny/Room1/BP_Shelf1_Donny.BP_Shelf1_Donny_C|GetCube _array_element)))) false false)))

(fn CloseShelf1Donny
  (for _array_element (Variables|Default|Getshelf_1_donny)
    (Transformation|SetWorldLocation (Variables|/Game/Items/Items_For_Donny/Room1/BP_Shelf1_Donny.BP_Shelf1_Donny_C|GetCube _array_element) (Math|Vector|MakeVector (- (.x (Transformation|GetWorldLocation (Variables|/Game/Items/Items_For_Donny/Room1/BP_Shelf1_Donny.BP_Shelf1_Donny_C|GetCube _array_element))) 5e+01) (.y (Transformation|GetWorldLocation (Variables|/Game/Items/Items_For_Donny/Room1/BP_Shelf1_Donny.BP_Shelf1_Donny_C|GetCube _array_element))) (.z (Transformation|GetWorldLocation (Variables|/Game/Items/Items_For_Donny/Room1/BP_Shelf1_Donny.BP_Shelf1_Donny_C|GetCube _array_element)))) false false)))

(fn OpenShelf1Dick
  (bind _cube (Variables|Default|GetCube))
  (bind _returnvalue (Transformation|GetWorldLocation _cube))
  (Transformation|SetWorldLocation _cube (Math|Vector|MakeVector (+ (.x _returnvalue) 5e+01) (.y _returnvalue) (.z _returnvalue)) false false))

(fn OpenEvidence
  (bind _evidence (Variables|Default|GetEvidence))
  (bind _cube (Variables|/Game/Items/Items_For_Dick/Room1/BP_Evidence_Dick.BP_Evidence_Dick_C|GetCube _evidence))
  (bind _returnvalue (Transformation|GetWorldLocation _cube))
  (Transformation|SetWorldLocation _cube (Math|Vector|MakeVector (+ (.x _returnvalue) 5e+01) (.y _returnvalue) (.z _returnvalue)) false false))

(fn CloseShelf1Dick
  (bind _cube (Variables|Default|GetCube))
  (bind _returnvalue (Transformation|GetWorldLocation _cube))
  (Transformation|SetWorldLocation _cube (Math|Vector|MakeVector (- (.x _returnvalue) 5e+01) (.y _returnvalue) (.z _returnvalue)) false false))

(fn CloseEvidence
  (bind _evidence (Variables|Default|GetEvidence))
  (bind _cube (Variables|/Game/Items/Items_For_Dick/Room1/BP_Evidence_Dick.BP_Evidence_Dick_C|GetCube _evidence))
  (bind _returnvalue (Transformation|GetWorldLocation _cube))
  (Transformation|SetWorldLocation _cube (Math|Vector|MakeVector (- (.x _returnvalue) 5e+01) (.y _returnvalue) (.z _returnvalue)) false false))