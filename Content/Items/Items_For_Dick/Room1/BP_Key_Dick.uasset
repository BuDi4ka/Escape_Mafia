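; BP_Key_Dick is an interactable Room 1 key pickup for the BP_Dick player character.
; BeginPlay caches the player as BP_Dick.
; On interact, it loops over all actors tagged "key", destroying each, setting the player's HasKeyRoom1 flag and printing a pickup message.
; Each loop iteration also spawns a BP_AssetKey at a hardcoded world location.
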(event EventBeginPlay
  (bind _asbp_dick (Utilities|Casting|CastToBP_Dick (Game|GetPlayerCharacter 0)))
  (Variables|Default|Set%20BP%20Dick _asbp_dick))

(event EventOnInteract
  (params (InteractingPlayer :type Character%20Object%20Reference) (Player%20Index :type Integer))
  ;[1 1 1] On Interact
  (bind _outactors (Actor|GetAllActorswithTag "key"))
  (for _array_element _outactors
    (Actor|DestroyActor _array_element)
    (Variables|/Game/Character/Dick/BP_Dick.BP_Dick_C|SethasKeyRoom1? (Variables|Default|Get%20BP%20Dick) true)
    (Development|PrintString "KEY Picked Up" true true "(R=0.962579,G=1.000000,B=0.035516,A=1.000000)" 1e+01)
    (Game|SpawnActorfromClass "/Game/Items/Items_2D/Room1/BP_AssetKey.BP_AssetKey_C" (Math|Transform|MakeTransform "1600.000000,2785.933881,99.124176" "0, 0, 0" "1.000000,1.000000,1.000000") "Undefined" "MultiplyWithRoot" 0 0)))

(fn ConstructionScript
  (|CallParentFunction))