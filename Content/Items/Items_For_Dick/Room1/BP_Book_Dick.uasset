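; Interactable book pickup for the Dick character that, once collected, reveals Donny's arrow message and unlocks Dick's pneumatics.
; A fast looping timer shows the prompt widget and outline while interactable and prompted, and sphere overlap also toggles the outline.
; On interact it flags BookDestroyed on BP_Dick, hides the mesh and updates the tagged actors cached at BeginPlay.
; Actor destruction and Donny pneumatic recoloring are present but never run.
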(event OnComponentBeginOverlap(Sphere)
  (params (OverlappedComponent :type Primitive%20Component%20Object%20Reference) (OtherActor :type Actor%20Object%20Reference) (OtherComp :type Primitive%20Component%20Object%20Reference) (OtherBodyIndex :type Integer) (bFromSweep :type Boolean) (SweepResult :type Hit%20Result%20Structure%20%28by%20ref%29))
  (if (Variables|Default|GetInteractable)
    (Rendering|Material|SetOverlayMaterial (Variables|Default|GetCylinder) "/Game/Assets/Materials/M_Outline.M_Outline" :!class /Script/Engine.MeshComponent)))

(event OnComponentEndOverlap(Sphere)
  (params (OverlappedComponent :type Primitive%20Component%20Object%20Reference) (OtherActor :type Actor%20Object%20Reference) (OtherComp :type Primitive%20Component%20Object%20Reference) (OtherBodyIndex :type Integer))
  (Rendering|Material|SetOverlayMaterial (Variables|Default|GetCylinder) 0 :!class /Script/Engine.MeshComponent))

(event Custom|CheckWidget
  (bind _widget (Variables|Default|GetWidget))
  (if (and (Variables|Default|GetInteractable) (Variables|Default|GetisPrompt))
    (Rendering|SetVisibility _widget true false)
    (Rendering|Material|SetOverlayMaterial (Variables|Default|GetCylinder) "/Game/Assets/Materials/M_Outline.M_Outline" :!class /Script/Engine.MeshComponent)
    (else
      (Rendering|SetVisibility _widget false false))))

(event EventOnInteract
  (params (InteractingPlayer :type Character%20Object%20Reference) (Player%20Index :type Integer))
  (bind _asbp_dick (Utilities|Casting|CastToBP_Dick (Game|GetPlayerCharacter 0)))
  (Variables|/Game/Character/Dick/BP_Dick.BP_Dick_C|SetBookDestroyed _asbp_dick true)
  ;[1 1 1] On Interact
  (Variables|Default|SetDrawUI? true)
  (Rendering|SetVisibility (Variables|Default|GetCylinder) false false)
  (Variables|Default|SetInteractable false)
  (Variables|Default|SetisPrompt false)
  (Development|PrintString "BOOK PICKED UP" true true "(R=1.000000,G=0.805564,B=0.000000,A=1.000000)" 3.0)
  (for _array_element (Variables|Default|GetDonnyArrow)
    (Rendering|SetActorHiddenInGame _array_element false)
    ;[1 1 1] Changing colors for Pneumatics
    (for _array_element_2 (Variables|Default|Getdick_pneumatic)
      (Variables|/Game/Items/Items_For_Dick/Room1/BP_Pneumatic_Dick.BP_Pneumatic_Dick_C|SetInteractable _array_element_2 true))))

(event EventBeginPlay
  (Utilities|Time|SetTimerbyEvent (delegate Custom|CheckWidget) 0.01 true)
  (bind _outactors (Actor|GetAllActorsOfClasswithTag "/Game/Items/Items_For_Donny/Room1/BP_Donny_MessageForPneumatic.BP_Donny_MessageForPneumatic_C" "arrow"))
  (Variables|Default|SetDonnyArrow _outactors)
  ;[1 1 1] Getting Pneumatics
  (bind _outactors_2 (Actor|GetAllActorsOfClasswithTag "/Game/Items/Items_For_Dick/Room1/BP_Pneumatic_Dick.BP_Pneumatic_Dick_C" "dickpneumatic"))
  (Variables|Default|Setdick_pneumatic _outactors_2)
  (bind _outactors_3 (Actor|GetAllActorsOfClasswithTag "/Game/Items/Items_For_Donny/Room1/BP_Pneumatic_Donny.BP_Pneumatic_Donny_C" "donnypneumatic"))
  (Variables|Default|Setdonny_pneumatic _outactors_3))

(fn ConstructionScript
  (|CallParentFunction))