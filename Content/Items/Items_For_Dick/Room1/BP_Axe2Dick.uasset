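; BP_Axe2Dick is an axe item under Room1 that shakes when the player interacts with it.
; Interaction sets an Interacted flag and plays a timeline whose Shake track drives the mesh's relative roll, then clears the flag when finished.
; A sphere overlap applies an outline overlay material while the axe is Interactable and removes it when the overlap ends.
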(event OnComponentBeginOverlap(Sphere)
  (params (OverlappedComponent :type Primitive%20Component%20Object%20Reference) (OtherActor :type Actor%20Object%20Reference) (OtherComp :type Primitive%20Component%20Object%20Reference) (OtherBodyIndex :type Integer) (bFromSweep :type Boolean) (SweepResult :type Hit%20Result%20Structure%20%28by%20ref%29))
  (if (Variables|Default|GetInteractable)
    (Rendering|Material|SetOverlayMaterial (Variables|Default|GetAxe2) "/Game/Assets/Materials/M_Outline.M_Outline" :!class /Script/Engine.MeshComponent)))

(event OnComponentEndOverlap(Sphere)
  (params (OverlappedComponent :type Primitive%20Component%20Object%20Reference) (OtherActor :type Actor%20Object%20Reference) (OtherComp :type Primitive%20Component%20Object%20Reference) (OtherBodyIndex :type Integer))
  (Rendering|Material|SetOverlayMaterial (Variables|Default|GetAxe2) 0 :!class /Script/Engine.MeshComponent))

(event EventOnInteract
  (params (InteractingPlayer :type Character%20Object%20Reference) (Player%20Index :type Integer))
  (Variables|Default|SetInteracted true)
  (bind _shake (Timeline|Timeline PlayFromStart)
    (:Update
      (Transformation|SetRelativeRotation (Variables|Default|GetAxe2) (Math|Rotator|MakeRotator (* _shake 1.0) 0.0 0.0) false false))
    (:Finished
      (Variables|Default|SetInteracted false))))

(fn ConstructionScript
  (|CallParentFunction))