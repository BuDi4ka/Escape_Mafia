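; Interactable pneumatic object for Dick in Room 1 that reveals Donny's book when used.
; At BeginPlay it caches Donny's pneumatic actors and book items by class and tag, and starts a fast looping timer that shows the prompt widget only while interactable and prompted.
; Interacting unhides the books, turns this cube and Donny's pneumatic cubes gray, and disables further interaction, all inside the book loop.
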(event Custom|CheckWidget
  (bind _widget (Variables|Default|GetWidget))
  (if (and (Variables|Default|GetInteractable) (Variables|Default|GetisPrompt))
    (Rendering|SetVisibility _widget true false)
    (else
      (Rendering|SetVisibility _widget false false))))

(event EventOnInteract
  (params (InteractingPlayer :type Character%20Object%20Reference) (Player%20Index :type Integer))
  (for _array_element (Variables|Default|Getbook_donny)
    (Rendering|SetActorHiddenInGame _array_element false)
    (Rendering|Material|SetMaterial (Variables|Default|GetCube) 1 "/Game/Assets/3D_Rooms/Room_1/Gray.Gray")
    (Variables|Default|SetInteractable false)
    (Variables|Default|SetisPrompt false)
    (for _array_element_2 (Variables|Default|Getdonny_pneumatic)
      (Rendering|Material|SetMaterial (Variables|/Game/Items/Items_For_Donny/Room1/BP_Pneumatic_Donny.BP_Pneumatic_Donny_C|GetCube _array_element_2) 1 "/Game/Assets/3D_Rooms/Room_1/Gray.Gray"))))

(event EventBeginPlay
  (Utilities|Time|SetTimerbyEvent (delegate Custom|CheckWidget) 0.01 true)
  (bind _outactors (Actor|GetAllActorsOfClasswithTag "/Game/Items/Items_For_Donny/Room1/BP_Pneumatic_Donny.BP_Pneumatic_Donny_C" "donnypneumatic"))
  (Variables|Default|Setdonny_pneumatic _outactors)
  (bind _outactors_2 (Actor|GetAllActorsOfClasswithTag "/Game/Items/BP_Item.BP_Item_C" "book_donny"))
  (Variables|Default|Setbook_donny _outactors_2))

(fn ConstructionScript
  (|CallParentFunction))