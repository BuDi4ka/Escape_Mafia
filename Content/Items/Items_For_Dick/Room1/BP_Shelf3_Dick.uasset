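; Interactable shelf for Room 1 that slides back and forth along world Y each time it is used.
; A FlipFlop on OnInteract alternates between a negative and an equal positive offset, applied instantly to the Cube component.
; The referenced Book's Cylinder gets the same offset, so it travels with the shelf.
; IsInteractable always returns true.
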(event EventOnInteract
  (params (InteractingPlayer :type Character%20Object%20Reference))
  (bind _cube (Variables|Default|GetCube))
  (bind _cube_2 (Variables|Default|GetCube))
  (bind _book (Variables|Default|GetBook))
  (bind _book_2 (Variables|Default|GetBook))
  (bind _returnvalue (Transformation|GetWorldLocation _cube))
  (bind _returnvalue_2 (Transformation|GetWorldLocation _cube_2))
  (bind _cylinder (Variables|/Game/Items/Items_For_Intercom/Room1/BP_Book_ForIntercom.BP_Book_ForIntercom_C|GetCylinder _book))
  (bind _cylinder_2 (Variables|/Game/Items/Items_For_Intercom/Room1/BP_Book_ForIntercom.BP_Book_ForIntercom_C|GetCylinder _book_2))
  (bind _returnvalue_3 (Transformation|GetWorldLocation _cylinder))
  (bind _returnvalue_4 (Transformation|GetWorldLocation _cylinder_2))
  (Utilities|FlowControl|FlipFlop
    (:A
      (Transformation|SetWorldLocation _cube_2 (Math|Vector|MakeVector (.x _returnvalue_2) (- (.y _returnvalue_2) 1e+02) (.z _returnvalue_2)) false false)
      (Transformation|SetWorldLocation _cylinder (Math|Vector|MakeVector (.x _returnvalue_3) (- (.y _returnvalue_3) 1e+02) (.z _returnvalue_3)) false false))
    (:B
      (Transformation|SetWorldLocation _cube (Math|Vector|MakeVector (.x _returnvalue) (+ (.y _returnvalue) 1e+02) (.z _returnvalue)) false false)
      (Transformation|SetWorldLocation _cylinder_2 (Math|Vector|MakeVector (.x _returnvalue_4) (+ (.y _returnvalue_4) 1e+02) (.z _returnvalue_4)) false false))))

(fn ConstructionScript
  (|CallParentFunction))

(fn IsInteractable
  (return true))