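; Interactable left cupboard door that swings open and closed on alternating interactions.
; A FlipFlop plays or reverses a timeline that yaws the door and its widget up to 90 degrees.
; While the door is interactable and the player overlaps its sphere, a fast looping timer shows the widget and applies an outline overlay material.
; Sphere overlap events also toggle the outline.
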(event OnComponentBeginOverlap(Sphere)
  (params (OverlappedComponent :type Primitive%20Component%20Object%20Reference) (OtherActor :type Actor%20Object%20Reference) (OtherComp :type Primitive%20Component%20Object%20Reference) (OtherBodyIndex :type Integer) (bFromSweep :type Boolean) (SweepResult :type Hit%20Result%20Structure%20%28by%20ref%29))
  (if (Variables|Default|GetInteractable)
    (Rendering|Material|SetOverlayMaterial (Variables|Default|GetDoor) "/Game/Assets/Materials/M_Outline.M_Outline" :!class /Script/Engine.MeshComponent)))

(event OnComponentEndOverlap(Sphere)
  (params (OverlappedComponent :type Primitive%20Component%20Object%20Reference) (OtherActor :type Actor%20Object%20Reference) (OtherComp :type Primitive%20Component%20Object%20Reference) (OtherBodyIndex :type Integer))
  (Rendering|Material|SetOverlayMaterial (Variables|Default|GetDoor) 0 :!class /Script/Engine.MeshComponent))

(event Custom|CheckWidget
  (bind _door (Variables|Default|GetDoor))
  (if (and (Variables|Default|GetInteractable) (Collision|IsOverlappingActor (Variables|Default|GetSphere) (Game|GetPlayerCharacter 0) :!class /Script/Engine.PrimitiveComponent))
    (Rendering|SetVisibility (Variables|Default|GetWidget) true false)
    (Rendering|Material|SetOverlayMaterial _door "/Game/Assets/Materials/M_Outline.M_Outline" :!class /Script/Engine.MeshComponent)
    (else
      (Rendering|SetVisibility (Variables|Default|GetWidget) false false)
      (Rendering|Material|SetOverlayMaterial _door 0 :!class /Script/Engine.MeshComponent))))

(event EventOnInteract
  (params (InteractingPlayer :type Character%20Object%20Reference) (Player%20Index :type Integer))
  (Utilities|FlowControl|FlipFlop
    (:A
      (Variables|Default|SetInteracted true)
      (bind _open_close (Timeline|OpenCupboard Play)
        (:Update
          (Transformation|SetRelativeRotation (Variables|Default|GetDoor) (Math|Rotator|MakeRotator 0.0 0.0 (* _open_close -9e+01)) false false)
          (Transformation|SetRelativeRotation (Variables|Default|GetWidget) (Math|Rotator|MakeRotator 0.0 0.0 (* _open_close -9e+01)) false false))))
    (:B
      (Variables|Default|SetInteracted false)
      (Timeline|OpenCupboard Reverse))))

(event EventBeginPlay
  (Utilities|Time|SetTimerbyEvent (delegate Custom|CheckWidget) 0.01 true)
  (Variables|Default|SetWidgetOffset (Variables|/Script/Engine.SceneComponent|GetRelativeRotation (Variables|Default|GetWidget))))

(fn ConstructionScript
  (|CallParentFunction))