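; BP_Cypher_Dick is an interactable cypher pickup item for Room1.
; On interact, it destroys every actor tagged "cypher", printing a pickup message and spawning a BP_AssetCypher at a hardcoded world position for each one.
; While Interactable is set, entering the Sphere trigger applies the M_Outline overlay material to Sphere0, and leaving the trigger clears it.
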(event OnComponentBeginOverlap(Sphere)
  (params (OverlappedComponent :type Primitive%20Component%20Object%20Reference) (OtherActor :type Actor%20Object%20Reference) (OtherComp :type Primitive%20Component%20Object%20Reference) (OtherBodyIndex :type Integer) (bFromSweep :type Boolean) (SweepResult :type Hit%20Result%20Structure%20%28by%20ref%29))
  (if (Variables|Default|GetInteractable)
    (Rendering|Material|SetOverlayMaterial (Variables|Default|GetSphere_0) "/Game/Assets/Materials/M_Outline.M_Outline" :!class /Script/Engine.MeshComponent)))

(event OnComponentEndOverlap(Sphere)
  (params (OverlappedComponent :type Primitive%20Component%20Object%20Reference) (OtherActor :type Actor%20Object%20Reference) (OtherComp :type Primitive%20Component%20Object%20Reference) (OtherBodyIndex :type Integer))
  (Rendering|Material|SetOverlayMaterial (Variables|Default|GetSphere_0) 0 :!class /Script/Engine.MeshComponent))

(event EventOnInteract
  (params (InteractingPlayer :type Character%20Object%20Reference) (Player%20Index :type Integer))
  ;[1 1 1] On Interact
  (bind _outactors (Actor|GetAllActorswithTag "cypher"))
  (for _array_element _outactors
    (Actor|DestroyActor _array_element)
    (Development|PrintString "CYPHER PICKED UP" true true "(R=0.000000,G=1.000000,B=0.024614,A=1.000000)" 4.0)
    (Game|SpawnActorfromClass "/Game/Items/Items_2D/Room1/BP_AssetCypher.BP_AssetCypher_C" (Math|Transform|MakeTransform "1641.025655,2785.933881,99.124176" "0, 0, 0" "1.000000,1.000000,1.000000") "Undefined" "MultiplyWithRoot" 0 0)))

(fn ConstructionScript
  (|CallParentFunction))