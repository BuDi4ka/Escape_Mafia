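; BP_Door_Dick is a door actor that swings open once when OpenDoor is called.
; OpenDoor passes through a DoOnce, plays a big metal door sound and runs a timeline that lerps the Cube's relative yaw to the open angle.
; Tick keeps the widget facing the camera of player index 1, while OnInteract is left empty.
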(event Custom|OpenDoor
  (Utilities|FlowControl|DoOnce false
    (:Completed
      (Audio|PlaySound2D "/Game/Audio/SFX/opening_big_metal_door_sfx.opening_big_metal_door_sfx" 1.0 1.0 0.0 0 0)
      (bind _doorfloat (Timeline|OpenDoorTimeline Play)
        (:Update
          (Transformation|SetRelativeRotation (Variables|Default|GetCube) (Math|Rotator|MakeRotator 0.0 0.0 (Math|Float|Lerp 1e+01 9e+01 _doorfloat)) false false))))))

(event EventTick
  (params (DeltaSeconds :type Float%20%28single-precision%29))
  (bind _widget (Variables|Default|GetWidget))
  (Transformation|SetWorldRotation _widget (Math|Rotator|FindLookatRotation (Transformation|GetWorldLocation _widget) (Camera|GetCameraLocation (Game|GetPlayerCameraManager 1))) false false))

(event EventOnInteract
  (params (InteractingPlayer :type Character%20Object%20Reference) (Player%20Index :type Integer)))

(fn ConstructionScript
  (|CallParentFunction))