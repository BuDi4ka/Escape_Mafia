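; Interactable shelf in Room1 that opens and closes together with its paired BP_Shelf2_Donny shelves.
; BeginPlay caches the tagged Donny shelves and starts a fast looping timer that shows the prompt widget while Interactable and IsPrompt are true.
; Each interaction alternates through a FlipFlop, instantly shifting its own Cube and each Donny shelf's Cube a fixed distance along world X, out or back.
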(event Custom|CheckWidget
  (if (and (Variables|Default|GetInteractable) (Variables|Default|GetisPrompt))
    (Rendering|SetVisibility (Variables|Default|GetWidget) true false)))

(event EventBeginPlay
  (Utilities|Time|SetTimerbyEvent (delegate Custom|CheckWidget) 0.01 true)
  (bind _outactors (Actor|GetAllActorsOfClasswithTag "/Game/Items/Items_For_Donny/Room1/BP_Shelf2_Donny.BP_Shelf2_Donny_C" "shelf2donny"))
  (Variables|Default|Setshelf_2_donny _outactors))

(event EventOnInteract
  (params (InteractingPlayer :type Character%20Object%20Reference) (Player%20Index :type Integer))
  ;[1 1 1] On Interact
  (Utilities|FlowControl|FlipFlop
    (:A
      (CallFunction|OpenShelf2Dick)
      (CallFunction|OpenShelf2Donny))
    (:B
      (CallFunction|CloseShelf2Dick)
      (CallFunction|CloseShelf2Donny))))

(fn ConstructionScript
  (|CallParentFunction))

(fn OpenShelf2Dick
  (bind _cube (Variables|Default|GetCube))
  (bind _returnvalue (Transformation|GetWorldLocation _cube))
  (Transformation|SetWorldLocation _cube (Math|Vector|MakeVector (+ (.x _returnvalue) 5e+01) (.y _returnvalue) (.z _returnvalue)) false false))

(fn OpenShelf2Donny
  (for _array_element (Variables|Default|Getshelf_2_donny)
    (Transformation|SetWorldLocation (Variables|/Game/Items/Items_For_Donny/Room1/BP_Shelf2_Donny.BP_Shelf2_Donny_C|GetCube _array_element) (Math|Vector|MakeVector (+ (.x (Transformation|GetWorldLocation (Variables|/Game/Items/Items_For_Donny/Room1/BP_Shelf2_Donny.BP_Shelf2_Donny_C|GetCube _array_element))) 5e+01) (.y (Transformation|GetWorldLocation (Variables|/Game/Items/Items_For_Donny/Room1/BP_Shelf2_Donny.BP_Shelf2_Donny_C|GetCube _array_element))) (.z (Transformation|GetWorldLocation (Variables|/Game/Items/Items_For_Donny/Room1/BP_Shelf2_Donny.BP_Shelf2_Donny_C|GetCube _array_element)))) false false)))

(fn CloseShelf2Dick
  (bind _cube (Variables|Default|GetCube))
  (bind _returnvalue (Transformation|GetWorldLocation _cube))
  (Transformation|SetWorldLocation _cube (Math|Vector|MakeVector (- (.x _returnvalue) 5e+01) (.y _returnvalue) (.z _returnvalue)) false false))

(fn CloseShelf2Donny
  (for _array_element (Variables|Default|Getshelf_2_donny)
    (Transformation|SetWorldLocation (Variables|/Game/Items/Items_For_Donny/Room1/BP_Shelf2_Donny.BP_Shelf2_Donny_C|GetCube _array_element) (Math|Vector|MakeVector (- (.x (Transformation|GetWorldLocation (Variables|/Game/Items/Items_For_Donny/Room1/BP_Shelf2_Donny.BP_Shelf2_Donny_C|GetCube _array_element))) 5e+01) (.y (Transformation|GetWorldLocation (Variables|/Game/Items/Items_For_Donny/Room1/BP_Shelf2_Donny.BP_Shelf2_Donny_C|GetCube _array_element))) (.z (Transformation|GetWorldLocation (Variables|/Game/Items/Items_For_Donny/Room1/BP_Shelf2_Donny.BP_Shelf2_Donny_C|GetCube _array_element)))) false false)))