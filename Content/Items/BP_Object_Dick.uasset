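; BP_Object_Dick is an item Blueprint that clears its owning BP_Object_Donny's IsVisible flag when the player character touches it.
; On BeginPlay it caches the player character as BP_Character, then casts its owner to BP_Object_Donny and stores that too.
; Begin overlap on SphereCollisionDick compares the other actor to the cached character and, on a match, sets the flag to false.
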(event OnComponentBeginOverlap(SphereCollisionDick)
  (params (OverlappedComponent :type Primitive%20Component%20Object%20Reference) (OtherActor :type Actor%20Object%20Reference) (OtherComp :type Primitive%20Component%20Object%20Reference) (OtherBodyIndex :type Integer) (bFromSweep :type Boolean) (SweepResult :type Hit%20Result%20Structure%20%28by%20ref%29))
  (if (== OtherActor (Variables|Default|GetBP%20Character))
    (Variables|/Game/Items/BP_Object_Donny.BP_Object_Donny_C|SetisVisible (Variables|Default|GetBP%20Object%20Donny) false)))

(event EventBeginPlay
  (Utilities|FlowControl|Sequence
    (:then_0
      (bind _asbp_character (Utilities|Casting|CastToBP_Character (Game|GetPlayerCharacter 0)))
      (Variables|Default|SetBP%20Character _asbp_character))
    (:then_1
      (bind _asbp_object_donny (Utilities|Casting|CastToBP_Object_Donny (Components|GetOwner)))
      (Variables|Default|SetBP%20Object%20Donny _asbp_object_donny))))

(fn ConstructionScript)