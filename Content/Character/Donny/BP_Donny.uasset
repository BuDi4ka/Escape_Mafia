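; BP_Donny is a first-person player character that sets up its own HUD and camera pitch limits, then caches tagged book and crystal actors.
; Book and crystal inputs, gated by destroyed flags, flip-flop overlay widgets and lock movement and look on hardcoded player controller 1.
; Pressing the crystal input once it is destroyed also unlocks jumping.
; An item-detection sphere trace exists, but its looping timer is never started.
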(event Custom|CustomEvent
  (bind _firstpersoncamera (Variables|Default|GetFirstPersonCamera))
  (bind _returnvalue (Transformation|GetWorldLocation _firstpersoncamera))
  (bind _outhit (Collision|SphereTraceByChannel _returnvalue (+ _returnvalue (* (Math|Vector|GetForwardVector _firstpersoncamera) (Math|Float|MakeLiteralFloat 2.5e+02))) 5.0 "TraceTypeQuery1" false 0 "None" true "(R=1.000000,G=0.000000,B=0.000000,A=1.000000)" "(R=0.000000,G=1.000000,B=0.000000,A=1.000000)" 0.2))
  (bind _asbp_item (Utilities|Casting|CastToBP_Item (.HitActor (Collision|BreakHitResult _outhit)))))

(event Input|EnhancedActionEvents|EnhancedInputActionIA_Book
  (params (ActionValue :type Boolean) (ElapsedSeconds :type Float%20%28double-precision%29) (TriggeredSeconds :type Float%20%28double-precision%29) (InputAction :type Input%20Action%20Object%20Reference :default "/Game/Character/Input/Actions/IA_Book.IA_Book"))
  (bind _returnvalue (Game|GetPlayerController 1))
  (if (Variables|Default|GetBookDestroyed)
    (for _array_element (Variables|Default|GetBook%20Donny)
      (Utilities|IsValid _array_element
        (:Is%20Not%20Valid
          (Utilities|FlowControl|FlipFlop
            (:A
              (bind _returnvalue_2 (UserInterface|CreateWidget "/Game/UI/WBP/WBP_Donny_Book.WBP_Donny_Book_C" _returnvalue))
              (UserInterface|Viewport|AddtoPlayerScreen _returnvalue_2)
              (Input|SetIgnoreMoveInput _returnvalue true)
              (Input|SetIgnoreLookInput _returnvalue true)
              (Utilities|FlowControl|Delay 0.15))
            (:B
              (Widget|RemovefromParent _returnvalue_2)
              (Input|SetIgnoreMoveInput _returnvalue false)
              (Input|SetIgnoreLookInput _returnvalue false)
              (Utilities|FlowControl|Delay 0.15)
              (Variables|Default|SetisUIopened false))))))))

(event Input|EnhancedActionEvents|EnhancedInputActionIA_Crystal
  (params (ActionValue :type Boolean) (ElapsedSeconds :type Float%20%28double-precision%29) (TriggeredSeconds :type Float%20%28double-precision%29) (InputAction :type Input%20Action%20Object%20Reference :default "/Game/Character/Input/Actions/IA_Crystal.IA_Crystal"))
  (bind _returnvalue (Game|GetPlayerController 1))
  (if (Variables|Default|GetCrystalDestroyed)
    (Variables|Default|SetisCrystalObserved true)
    (Development|PrintString "JUMPING ENABLED" true true "(R=1.000000,G=0.000000,B=0.971960,A=1.000000)")
    (for _array_element (Variables|Default|GetCrystalDonny)
      (Utilities|IsValid _array_element
        (:Is%20Not%20Valid
          (Utilities|FlowControl|FlipFlop
            (:A
              (bind _returnvalue_2 (UserInterface|CreateWidget "/Game/UI/WBP/WBP_Donny_Crystal.WBP_Donny_Crystal_C" _returnvalue))
              (UserInterface|Viewport|AddtoPlayerScreen _returnvalue_2)
              (Input|SetIgnoreMoveInput _returnvalue true)
              (Input|SetIgnoreLookInput _returnvalue true)
              (Utilities|FlowControl|Delay 0.15))
            (:B
              (Widget|RemovefromParent _returnvalue_2)
              (Input|SetIgnoreMoveInput _returnvalue false)
              (Input|SetIgnoreLookInput _returnvalue false)
              (Utilities|FlowControl|Delay 0.15)
              (Variables|Default|SetisUIopened false))))))))

(event Input|EnhancedActionEvents|EnhancedInputActionIA_Jump
  (params (ActionValue :type Boolean) (ElapsedSeconds :type Float%20%28double-precision%29) (TriggeredSeconds :type Float%20%28double-precision%29) (InputAction :type Input%20Action%20Object%20Reference :default "/Game/Character/Input/Actions/IA_Jump.IA_Jump"))
  (:Started
    (if (Variables|Default|GetisCrystalObserved)
      (Character|Jump)))
  (:Completed
    (Character|StopJumping)))

(event EventBeginPlay
  (bind _player_index (Variables|Default|Getplayer_index))
  (bind _returnvalue (Game|GetPlayerCameraManager _player_index))
  (bind _returnvalue_2 (UserInterface|CreateWidget "/Game/UI/WBP/WBP_PlayersUI_Donny.WBP_PlayersUI_Donny_C" (Game|GetPlayerController _player_index)))
  (UserInterface|Viewport|AddtoPlayerScreen _returnvalue_2)
  (Variables|/Script/Engine.PlayerCameraManager|SetViewPitchMax _returnvalue 3e+01)
  (Variables|/Script/Engine.PlayerCameraManager|SetViewPitchMin _returnvalue -65.0)
  (bind _outactors (Actor|GetAllActorsOfClasswithTag "/Game/Items/Items_For_Donny/Room1/BP_Book_Donny.BP_Book_Donny_C" "book_donny"))
  (Variables|Default|SetBook%20Donny _outactors)
  (bind _outactors_2 (Actor|GetAllActorsOfClasswithTag "/Game/Items/Items_For_Donny/Room1/BP_Crystal_Donny.BP_Crystal_Donny_C" "crystal_donny"))
  (Variables|Default|SetCrystalDonny _outactors_2))

(fn ConstructionScript
  (|CallParentFunction))